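; Base game mode for all levels of a ball-shooting game, handling camera follow, stroke count and level completion.
; BeginPlay finds the level index, caches the player ball, camera and skybox, adds the aim-line widget and binds shoot and goal events.
; Tick nudges the camera on X and Z only when the ball leaves a bounding box, then snaps the skybox to it.
; GoalReached shows the completion widget.
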(event `self.ReceiveBeginPlay`
  (bind _returnvalue (`GameplayStatics.GetCurrentLevelName` true))
  (set `self.Level Index` (`KismetArrayLibrary.Array_Find` (`self.Levels`) _returnvalue)) ; Helps track the current level index for\nthe next button when goal is reached
  (bind _asplayer_ball_pawn_bp (cast `/Game/Blueprints/PlayerBallPawn_BP` (`GameplayStatics.GetPlayerPawn` 0)))
  (bind _output_get (set `self.Player Ball` _asplayer_ball_pawn_bp))
  (add `/Game/Blueprints/PlayerBallPawn_BP.OnPlayerBallShoot` _output_get (`|CreateDelegate` :!event `UpdateStrokeCount`))
  (bind _returnvalue_2 (`GameplayStatics.GetActorOfClass` "/Script/Engine.CameraActor"))
  (set `self.Camera` _returnvalue_2)
  (bind _returnvalue_3 (`GameplayStatics.GetActorOfClass` "/Game/Blueprints/Skybox_BP.Skybox_BP_C"))
  (set `self.SkyBox` _returnvalue_3)
  (bind _returnvalue_4 (`|CreateWidget` "/Game/Blueprints/UI/AimLine_BP.AimLine_BP_C"))
  (`UserWidget.AddToViewport` _returnvalue_4 0)
  (bind _returnvalue_5 (`GameplayStatics.GetActorOfClass` "/Game/Blueprints/Goal_BP.Goal_BP_C"))
  (add `/Game/Blueprints/Goal_BP.BallReached` _returnvalue_5 (`|CreateDelegate` :!event `GoalReached`)))

(event `self.ReceiveTick`
  (params (DeltaSeconds :type "Float (single-precision)"))
  (if (and (!= (`self.Camera`) null) (!= (`self.Player Ball`) null))
    (`self.MoveCamera`) ; Moves camera towards the player with a\nbounding box size of 620x360 using variables\nX Max and Z Max, where:\n\nX Max = 620 / 2 = 310\nZ Max = 360 / 2 = 180
    (`self.MoveSky`) ; Ensures Skybox follows the camera
  ))

(fn `GoalReached`
  (set `self.Goal Reached` true)
  (bind _returnvalue (`|CreateWidget` "/Game/Blueprints/UI/Goal_Reached_BP.Goal_Reached_BP_C"))
  (`UserWidget.AddToViewport` _returnvalue 0))

(fn `MoveCamera`
  (bind _camera (`self.Camera`))
  (bind _x_max (`self.X Max`))
  (bind _z_max (`self.Z Max`))
  (bind _rootcomponent (`Actor.RootComponent` _camera))
  (bind _returnvalue (- (`self.K2_GetActorLocation` (`self.Player Ball`)) (`self.K2_GetActorLocation` _camera)))
  (bind _returnvalue_2 (`KismetMathLibrary.Vector_GetAbs` _returnvalue))
  (bind (_returnvalue_x _returnvalue_y _returnvalue_z) (`KismetMathLibrary.BreakVector` (* (`KismetMathLibrary.Vector_GetSignVector` _returnvalue) (- _returnvalue_2 (`KismetMathLibrary.MakeVector` _x_max 0.0 _z_max)))))
  (if (> (.x _returnvalue_2) _x_max)
    (`SceneComponent.K2_AddWorldOffset` _rootcomponent (`KismetMathLibrary.MakeVector` _returnvalue_x) false false))
  (if (> (.z _returnvalue_2) _z_max)
    (`SceneComponent.K2_AddWorldOffset` _rootcomponent (`KismetMathLibrary.MakeVector` 0.0 0.0 _returnvalue_z) false false)))

(fn `MoveSky`
  (bind _skybox (`self.SkyBox`))
  (bind (_returnvalue_x _returnvalue_y _returnvalue_z) (`KismetMathLibrary.BreakVector` (- (`SceneComponent.K2_GetComponentLocation` (`CameraActor.CameraComponent` (`self.Camera`))) (`self.K2_GetActorLocation` _skybox))))
  (`SceneComponent.K2_AddWorldOffset` (`Actor.RootComponent` _skybox) (`KismetMathLibrary.MakeVector` _returnvalue_x 0.0 _returnvalue_z) false false) ; Ensures Sky follows camera in the X and Z Axis
)

(fn `UpdateStrokeCount`
  (set `self.StrokeCount` (+ (`self.StrokeCount`) 1))
  (return))

(fn `UserConstructionScript`)
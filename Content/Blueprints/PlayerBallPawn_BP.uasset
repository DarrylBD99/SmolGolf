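; Player golf ball pawn that is launched by swings and can show a predicted trajectory while aiming.
; On BeginPlay it binds to the player controller's swing and aim events.
; Swings apply a mass-scaled impulse and broadcast a shoot event, while aiming draws an optional debug-drawn projectile prediction with tuned gravity.
; Hits add manual friction force against horizontal velocity, working around physics-material friction on round collision shapes.
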(event `self.ReceiveBeginPlay`
  (bind _asplayer_controller_bp (cast `/Game/Blueprints/PlayerController_BP` (`GameplayStatics.GetPlayerController` 0)))
  (bind _output_get (set `self.Player Controller` _asplayer_controller_bp))
  (add `/Game/Blueprints/PlayerController_BP.OnBallSwing` _output_get (`|CreateDelegate` :!event `BallSwing`))
  (add `/Game/Blueprints/PlayerController_BP.OnBallAim` _output_get (`|CreateDelegate` :!event `GuideLine`)))

(event `self.ball_Sprite.OnComponentHit`
  (params (HitComponent :type "PrimitiveComponent Object Reference") (OtherActor :type "Actor Object Reference") (OtherComp :type "PrimitiveComponent Object Reference") (NormalImpulse :type "Vector Structure") (Hit :type "HitResult Structure (by ref)"))
  (bind (_returnvalue_x _returnvalue_y) (`KismetMathLibrary.BreakVector` (`KismetMathLibrary.NegateVector` (`self.GetVelocity`))))
  (`PrimitiveComponent.AddForce` (`self.ball_Sprite`) (* (`PhysicalMaterial.Friction` (`.PhysMat` (`GameplayStatics.BreakHitResult` Hit))) (`KismetMathLibrary.MakeVector` _returnvalue_x _returnvalue_y)) "None" false) ; Due to friction in Physics Material only working well with cubes and\nnot circle/sphere collision shapes, it is required to add additional\ncode to apply friction to the golf ball manually.\n\nSource: https://forums.unrealengine.com/t/2017662
)

(fn `BallSwing`
  (params (AimVelocity :type "Vector Structure"))
  (bind _ball_sprite (`self.ball_Sprite`))
  (`PrimitiveComponent.AddImpulse` _ball_sprite (/ AimVelocity (`PrimitiveComponent.GetMass` _ball_sprite)) "None" false)
  (`self.OnPlayerBallShoot`)
  (return))

(fn `GuideLine`
  (params (AimVelocity :type "Vector Structure"))
  (bind _returnvalue (`PrimitiveComponent.GetMass` (`self.ball_Sprite`)))
  (if (`self.GuideLineEnabled`)
    (`GameplayStatics.Blueprint_PredictProjectilePath_ByTraceChannel` (`self.K2_GetActorLocation`) (/ AimVelocity _returnvalue) true 2.0 "ECC_PhysicsBody" false (`|MakeArray` self :!type "Actor Object Reference") "ForOneFrame" 0.0 10.0 2.5 (* (* _returnvalue -980.0) 0.53))))

(fn `UserConstructionScript`)
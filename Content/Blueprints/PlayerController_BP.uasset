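; Player controller for a ball-swing level game that turns mouse drags into aim and swing events for the player ball, and handles level reset and main menu input.
; Until the goal is reached, Tick shows the cursor only while the ball is nearly still, which gates swing input.
; Dragging broadcasts a world-space aim vector and screen points for the aim line; release broadcasts the swing and disposes the line.
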(event `self.ReceiveTick`
  (params (DeltaSeconds :type "Float (single-precision)"))
  (bind _aslevel_gmb_bp (cast `/Game/Blueprints/Level_GMB_BP` (`GameplayStatics.GetGameMode`)))
  (if (not (`/Game/Blueprints/Level_GMB_BP.Goal Reached` _aslevel_gmb_bp))
    (set `self.bShowMouseCursor` (== (`self.GetVelocity` (stale `self.ReceiveBeginPlay` _output_get)) (`KismetMathLibrary.Conv_DoubleToVector` 0.0) :`ErrorTolerance` 1.0)) ; Ensures mouse cursor is only visible when the player\nball is not moving (or ball movement is minimal)
  ))

(event `self.ReceiveBeginPlay`
  (`EnhancedInputSubsystemInterface.AddMappingContext` (subsystem `EnhancedInputLocalPlayerSubsystem`) "/Game/Input/IMC.IMC" 0 (struct))
  (bind _returnvalue (`GameplayStatics.GetActorOfClass` "/Game/Blueprints/PlayerBallPawn_BP.PlayerBallPawn_BP_C"))
  (bind _output_get (set `self.Player Ball` _returnvalue)))

(event `EnhancedInput|/Game/Input/BallSwing_IA`
  (params (ActionValue :type Boolean) (ElapsedSeconds :type "Float (double-precision)") (TriggeredSeconds :type "Float (double-precision)") (InputAction :type "InputAction Object Reference" :default "/Game/Input/BallSwing_IA.BallSwing_IA"))
  (bind _worldlocation (`self.DeprojectMousePositionToWorld`))
  (bind _bshowmousecursor (`self.bShowMouseCursor`))
  (:`Started`
    (if _bshowmousecursor
      (set `self.BallSwingStarted` true :!label _label)
      (bind _returnvalue (`WidgetLayoutLibrary.GetMousePositionOnViewport`))
      (bind _output_get (set `self.MouseStartPos` _worldlocation))))
  (:`Ongoing`
    (if _bshowmousecursor
      (if (`self.BallSwingStarted`)
        (bind _returnvalue_2 (`WidgetLayoutLibrary.GetMousePositionOnViewport`))
        (`self.OnBallAimWidget` _returnvalue _returnvalue_2)
        (bind _returnvalue_3 (- _output_get _worldlocation))
        (`self.OnBallAim` _returnvalue_3)
        (else
          (goto _label)))))
  (:`Canceled`
    (if _bshowmousecursor :!label _label_2
      (set `self.BallSwingStarted` false)
      (`self.OnBallSwing` _returnvalue_3)
      (`self.BallAimLineDispose`)))
  (:`Completed`
    (goto _label_2)))

(event `EnhancedInput|/Game/Input/Reset_IA`
  (params (ActionValue :type Boolean) (ElapsedSeconds :type "Float (double-precision)") (TriggeredSeconds :type "Float (double-precision)") (InputAction :type "InputAction Object Reference" :default "/Game/Input/Reset_IA.Reset_IA"))
  (:`Triggered`
    (bind _returnvalue (`GameplayStatics.GetCurrentLevelName` true))
    (`GameplayStatics.OpenLevel` (`KismetStringLibrary.Conv_StringToName` _returnvalue))))

(event `EnhancedInput|/Game/Input/MainMenu_IA`
  (params (ActionValue :type Boolean) (ElapsedSeconds :type "Float (double-precision)") (TriggeredSeconds :type "Float (double-precision)") (InputAction :type "InputAction Object Reference" :default "/Game/Input/MainMenu_IA.MainMenu_IA"))
  (:`Triggered`
    (`GameplayStatics.OpenLevel` "MainMenu")))

(fn `UserConstructionScript`)